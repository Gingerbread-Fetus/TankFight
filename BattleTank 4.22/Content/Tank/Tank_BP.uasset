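; Player-controllable tank Blueprint that aims, fires and drives on two tracks.
; BeginPlay registers the barrel and turret and initialises TankMovement with both tracks.
; Input rotates the azimuth gimbal and spring arm for aiming, calls Fire, and drives either through direct per-track throttles or TankMovement's forward and turn intents.
; The construction script assigns track and barrel meshes plus a physical material override on the tracks.
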(event `self.ReceiveBeginPlay`
  (`self.SetBarrelReference` (`self.Barrel`))
  (`self.SetTurretReference` (`self.TankTurret`))
  (`TankMovementComponent.Initialise` (`self.TankMovement`) (`self.Left Track`) (`self.Right Track`)))

(event `InputAction|Fire`
  (params (Key :type "Key Structure"))
  (:`Pressed`
    (`self.Fire`)))

(event `InputAxis|AimAzimuth`
  (params (AxisValue :type "Float (single-precision)"))
  ;[1 1 1] Aim Input Binding
  (`SceneComponent.K2_AddLocalRotation` (`self.AzimuthGimble`) (`KismetMathLibrary.MakeRotator` 0.0 0.0 AxisValue) false false))

(event `InputAxis|AimElevation`
  (params (AxisValue :type "Float (single-precision)"))
  ;[1 1 1] Aim Input Binding
  (`SceneComponent.K2_AddLocalRotation` (`self.SpringArm`) (`KismetMathLibrary.MakeRotator` 0.0 AxisValue) false false))

(event `InputAxis|Left Track Throttle`
  (params (AxisValue :type "Float (single-precision)"))
  ;[1 1 1] Movement Input Binding
  (`Tracks.SetThrottle` (`self.Left Track`) AxisValue))

(event `InputAxis|Right Track Throttle`
  (params (AxisValue :type "Float (single-precision)"))
  ;[1 1 1] Movement Input Binding
  (`Tracks.SetThrottle` (`self.Right Track`) AxisValue))

(event `InputAxis|Move Forward`
  (params (AxisValue :type "Float (single-precision)"))
  ;[1 1 1] Movement Input Binding
  (`TankMovementComponent.IntendMoveForward` (`self.TankMovement`) AxisValue))

(event `InputAxis|Turn Right`
  (params (AxisValue :type "Float (single-precision)"))
  ;[1 1 1] Movement Input Binding
  (`TankMovementComponent.IntendTurnRight` (`self.TankMovement`) AxisValue))

(fn `UserConstructionScript`
  (`StaticMeshComponent.SetStaticMesh` (`self.Right Track`) "/Game/Tank/tank_fbx_Track.tank_fbx_Track")
  (`StaticMeshComponent.SetStaticMesh` (`self.Left Track`) "/Game/Tank/tank_fbx_Track.tank_fbx_Track")
  (`StaticMeshComponent.SetStaticMesh` (`self.Barrel`) "/Game/Tank/tank_fbx_Barrel.tank_fbx_Barrel")
  (`PrimitiveComponent.SetPhysMaterialOverride` (`self.Left Track`) "/Game/Tank/Track.Track")
  (`PrimitiveComponent.SetPhysMaterialOverride` (`self.Right Track`) "/Game/Tank/Track.Track"))